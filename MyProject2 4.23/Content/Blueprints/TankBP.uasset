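; Player-controlled tank Blueprint that maps input to camera aiming, track driving and firing.
; On BeginPlay it passes the barrel and turret components to their reference setters, posts the TurretStartMove Wwise event and sets its Ak component as listener.
; Aim axes rotate the azimuth gimbal and spring arm, with an inverted elevation option.
; Separate throttle axes feed each track's C++ SetThrottle, and the Fire action calls Fire.
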(event `self.ReceiveBeginPlay`
  (bind _ak (`self.Ak`))
  (`self.SetBarrelReference` (`self.TankBarrel`))
  (`self.SetTurretReference` (`self.TankTurret`))
  (`AkGameplayStatics.PostEvent` "/Game/Audio/WwiseEvents/TurretStartMove.TurretStartMove" self)
  (`AkComponent.SetListeners` _ak (`|MakeArray` _ak)))

(event `self.WwisePostEvent`)

(event `InputAxis|AimAzimuth`
  (params (AxisValue :type "Float (single-precision)"))
  ;[1 1 1] Aiming
  (`SceneComponent.K2_AddLocalRotation` (`self.AzimuthGimbal`) (`KismetMathLibrary.MakeRotator` 0.0 0.0 AxisValue) false false))

(event `InputAxis|AimElevation`
  (params (AxisValue :type "Float (single-precision)"))
  ;[1 1 1] Aiming
  (`SceneComponent.K2_AddLocalRotation` (`self.SpringArm`) (`KismetMathLibrary.MakeRotator` 0.0 AxisValue) false false))

(event `InputAxis|LeftTrackThrottle`
  (params (AxisValue :type "Float (single-precision)"))
  (`TankTrack.setThrottle` (`self.LeftTrack`) AxisValue) ; Notice here that I created 'Blueprint callable' function in C++, that takes a float\nas an argumet. Now I can have this node in Blueprint (and when I search for it \nI can select which instantiation of it (here left track or right track) and it has a\nfloat input pin for the argument.
)

(event `InputAxis|RightTrackThrottle`
  (params (AxisValue :type "Float (single-precision)"))
  (`TankTrack.setThrottle` (`self.RightTrack`) AxisValue))

(event `InputAxis|AimElevationInvert`
  (params (AxisValue :type "Float (single-precision)"))
  ;[1 1 1] Aiming
  (`SceneComponent.K2_AddLocalRotation` (`self.SpringArm`) (`KismetMathLibrary.MakeRotator` 0.0 (* AxisValue -1.0)) false false))

(event `InputAction|Fire`
  (params (Key :type "Key Structure"))
  (:`Pressed`
    (`self.Fire`)))

(fn `UserConstructionScript`)